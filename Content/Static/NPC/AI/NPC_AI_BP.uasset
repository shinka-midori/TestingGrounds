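; AI controller for guard NPCs that switches their behavior tree between patrol and reacting to the player.
; On BeginPlay it initializes the PatrolData blackboard and runs the GuardBehaviour tree.
; Each tick it reads IsSensed on the controlled Ue4ASP_Character and sets the player pawn as the blackboard enemy, or clears that key when not sensed.
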(event EventBeginPlay
  (bind _blackboardcomponent (Class|AIController|UseBlackboard "/Game/Static/NPC/AI/PatrolData.PatrolData"))
  (AI|RunBehaviorTree "/Game/Static/NPC/AI/GuardBehaviour.GuardBehaviour"))

(event EventTick
  (params (DeltaSeconds :type Float%20%28single-precision%29))
  (bind _enemy_key (Variables|Default|GetEnemy%20Key))
  (bind _asue_4asp_character (Utilities|Casting|CastToUe4ASP_Character (Pawn|GetControlledPawn)))
  (if (Variables|/Game/Static/NPC/Behaviour/Ue4ASP_Character.Ue4ASP_Character_C|GetIs%20Sensed _asue_4asp_character)
    (AI|Components|Blackboard|SetValueasObject (stale EventBeginPlay _blackboardcomponent) _enemy_key (Game|Player|GetPlayerPawn 0))
    (else
      (AI|Components|Blackboard|ClearValue (stale EventBeginPlay _blackboardcomponent) _enemy_key))))

(fn ConstructionScript)
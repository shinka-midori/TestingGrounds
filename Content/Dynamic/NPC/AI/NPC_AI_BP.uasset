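; AI controller for guard NPCs that starts the GuardBehaviour behavior tree on the PatrolData blackboard.
; Each tick it casts the controlled pawn to ThirdPersonCharacter and skips any tagged Enemy.
; For the others, it polls the pawn's IsSensed flag, writing player pawn 0 to the EnemyKey blackboard value when set and clearing it otherwise.
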(event EventBeginPlay
  (bind _blackboardcomponent (Class|AIController|UseBlackboard "/Game/Dynamic/NPC/AI/PatrolData.PatrolData"))
  (AI|RunBehaviorTree "/Game/Dynamic/NPC/AI/GuardBehaviour.GuardBehaviour"))

(event EventTick
  (params (DeltaSeconds :type Float%20%28single-precision%29))
  (bind _enemy_key (Variables|Default|GetEnemy%20Key))
  (bind _asthird_person_character (Utilities|Casting|CastToThirdPersonCharacter (Pawn|GetControlledPawn)))
  (if (not (Actor|ActorHasTag _asthird_person_character "Enemy"))
    (if (Variables|/Game/Dynamic/NPC/Behaviour/ThirdPersonCharacter.ThirdPersonCharacter_C|GetIs%20Sensed _asthird_person_character)
      (AI|Components|Blackboard|SetValueasObject (stale EventBeginPlay _blackboardcomponent) _enemy_key (Game|Player|GetPlayerPawn 0))
      (else
        (AI|Components|Blackboard|ClearValue (stale EventBeginPlay _blackboardcomponent) _enemy_key)))))

(fn ConstructionScript)
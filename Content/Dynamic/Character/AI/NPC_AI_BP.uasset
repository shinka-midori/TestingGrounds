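; AI controller for guard NPCs that tells the behavior tree when the player is an enemy target.
; On BeginPlay it sets up the PatrolData blackboard and runs the GuardBehaviour tree.
; Each Tick it polls IsSensed on the controlled BP_Character, writing player character 0 to EnemyKey when true and clearing the key otherwise.
; The controller does no sensing itself and only relays that flag to the blackboard.
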(event EventBeginPlay
  (bind _blackboardcomponent (Class|AIController|UseBlackboard "/Game/Dynamic/Character/AI/PatrolData.PatrolData"))
  (AI|RunBehaviorTree "/Game/Dynamic/Character/AI/GuardBehaviour.GuardBehaviour"))

(event EventTick
  (params (DeltaSeconds :type Float%20%28single-precision%29))
  (bind _enemy_key (Variables|Default|GetEnemy%20Key))
  (bind _asbp_character (Utilities|Casting|CastToBP_Character (Pawn|GetControlledPawn)))
  (if (Variables|/Game/Dynamic/Character/Behaviour/BP_Character.BP_Character_C|GetIs%20Sensed _asbp_character)
    (AI|Components|Blackboard|SetValueasObject (stale EventBeginPlay _blackboardcomponent) _enemy_key (Game|GetPlayerCharacter 0))
    (else
      (AI|Components|Blackboard|ClearValue (stale EventBeginPlay _blackboardcomponent) _enemy_key))))

(fn ConstructionScript)
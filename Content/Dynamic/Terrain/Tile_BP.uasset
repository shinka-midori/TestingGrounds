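; Terrain tile actor with a barrier wall that opens while something overlaps the tile.
; It starts locked on BeginPlay; any actor overlap unlocks it and any end overlap locks it again, without filtering or counting actors.
; Lock and Unlock toggle the wall's collision and swap its material between red and green.
; GetAttachLocation exposes an Arrow component's world transform, apparently as an attach point.
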(event EventBeginPlay
  (CallFunction|Lock))

(event Collision|EventActorBeginOverlap
  (params (OtherActor :type Actor%20Object%20Reference))
  (CallFunction|Unlock))

(event EventTick
  (params (DeltaSeconds :type Float%20%28single-precision%29)))

(event Collision|EventActorEndOverlap
  (params (OtherActor :type Actor%20Object%20Reference))
  (CallFunction|Lock))

(fn ConstructionScript)

(fn GetAttachLocation
  (return (Transformation|GetWorldTransform (Variables|Default|GetArrow))))

(fn Unlock
  (Collision|SetCollisionEnabled (Variables|Default|GetBarrierWall) "NoCollision")
  (Rendering|Material|SetMaterial (Variables|Default|GetBarrierWall) 0 "/Game/Dynamic/Terrain/GreenBarrier.GreenBarrier"))

(fn Lock
  (Collision|SetCollisionEnabled (Variables|Default|GetBarrierWall) "QueryAndPhysics")
  (Rendering|Material|SetMaterial (Variables|Default|GetBarrierWall) 0 "/Game/Dynamic/Terrain/RedBarrier.RedBarrier"))
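; Game mode for an infinite terrain game that spawns chained tiles and keeps the player's score.
; BeginPlay runs two passes, each spawning a BP_Tile and calling PopulateBoundsVolumePool.
; SpawnTile hands each tile the shared NavMeshBoundsVolume pool, then stores its attach location as the next spawn transform.
; NewTileConquered increments the score, which GetScore exposes; it does not spawn tiles itself.
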(event EventBeginPlay
  (for _index (range 0 1)
    (CallFunction|SpawnTile)
    (Class|InfiniteTerrainGameMode|PopulateBoundsVolumePool)))

(event EventTick
  (params (DeltaSeconds :type Float%20%28single-precision%29)))

(fn ConstructionScript)

(fn SpawnTile
  (bind _returnvalue (Game|SpawnActorfromClass "/Game/Dynamic/Terrain/BP_Tile.BP_Tile_C" (Variables|Default|GetNext%20Tile%20Transform) "Undefined" 0 0))
  (Class|Tile|SetPool _returnvalue (Variables|Default|GetNavMeshBoundsVolumePool))
  (bind _attachtransform (Default|GetAttachLocation _returnvalue))
  (Variables|Default|SetNext%20Tile%20Transform _attachtransform))

(fn NewTileConquered
  (Math|Integer|IncrementInt (Variables|Default|GetScore)))

(fn GetScore
  (return (Variables|Default|GetScore)))